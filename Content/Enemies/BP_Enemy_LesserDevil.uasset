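; Flying lesser devil enemy that alternates between climbing and diving at the player, dealing damage on capsule contact.
; While DebugStopMovement is true, Tick faces the player; the charging phase feeds the player's offset world position as movement direction until height is reached.
; It then pauses, snapshots the player's location and dives toward it.
; On reaching that height it stops, re-enters charging and clears DebugStopMovement.
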(event `self.ReceiveBeginPlay`
  (`parent.ReceiveBeginPlay`)
  (`CharacterMovementComponent.SetMovementMode` (`self.CharacterMovement`) "MOVE_Flying" 0))

(event `self.ReceiveTick`
  (params (DeltaSeconds :type "Float (single-precision)"))
  (bind (_returnvalue_x _returnvalue_y _returnvalue_z) (`KismetMathLibrary.BreakVector` (`self.K2_GetActorLocation`)))
  (bind (_returnvalue_x_2 _returnvalue_y_2 _returnvalue_z_2) (`KismetMathLibrary.BreakVector` (`self.K2_GetActorLocation`)))
  (bind (_setplayerlocation_x _setplayerlocation_y _setplayerlocation_z) (`KismetMathLibrary.BreakVector` (`self.SetPlayerLocation`)))
  (bind _maxheight (`self.MaxHeight`))
  (bind (_returnvalue_roll _returnvalue_pitch _returnvalue_yaw) (`KismetMathLibrary.BreakRotator` (`KismetMathLibrary.FindLookAtRotation` (`self.K2_GetActorLocation`) (`self.K2_GetActorLocation` (`GameplayStatics.GetPlayerCharacter` 0)))))
  (bind (_returnvalue_x_3 _returnvalue_y_3 _returnvalue_z_3) (`KismetMathLibrary.BreakVector` (+ (`self.K2_GetActorLocation` (`GameplayStatics.GetPlayerCharacter` 0)) (`KismetMathLibrary.MakeVector` _maxheight _maxheight _maxheight))))
  (if (`self.DebugStopMovement`)
    (`self.K2_SetActorRotation` (`KismetMathLibrary.MakeRotator` 0.0 0.0 _returnvalue_yaw))
    (if (`self.bIsCharging`)
      (set `self.MaxSpeed` 0.01)
      (`self.AddMovementInput` (`KismetMathLibrary.MakeVector` _returnvalue_x_3 _returnvalue_y_3 _returnvalue_z_3) (`self.MaxSpeed`))
      (if (<= _returnvalue_z_3 _returnvalue_z_2)
        (`MovementComponent.StopMovementImmediately` (`self.CharacterMovement`))
        (`KismetSystemLibrary.Delay` 0.2)
        (set `self.bIsCharging` false)
        (set `self.SetPlayerLocation` (`self.K2_GetActorLocation` (`GameplayStatics.GetPlayerCharacter` 0))))
      (else
        (set `self.MaxSpeed` 10.0)
        (`self.AddMovementInput` (`KismetMathLibrary.Normal` (- (`self.SetPlayerLocation`) (`self.K2_GetActorLocation`))) (`self.MaxSpeed`) true)
        (if (>= _setplayerlocation_z _returnvalue_z)
          (`MovementComponent.StopMovementImmediately` (`self.CharacterMovement`))
          (set `self.DebugStopMovement` false)
          (set `self.bIsCharging` true))))))

(event `self.Capsule.OnComponentBeginOverlap`
  (params (OverlappedComponent :type "PrimitiveComponent Object Reference") (OtherActor :type "Actor Object Reference") (OtherComp :type "PrimitiveComponent Object Reference") (OtherBodyIndex :type Integer) (bFromSweep :type Boolean) (SweepResult :type "HitResult Structure (by ref)"))
  (bind _returnvalue (`GameplayStatics.GetPlayerCharacter` 0))
  (if (`GameplayStatics.ObjectIsA` OtherActor (`GameplayStatics.GetObjectClass` _returnvalue))
    (`GameplayStatics.ApplyDamage` _returnvalue 1.0)))

(fn `UserConstructionScript`
  (`parent.UserConstructionScript`))