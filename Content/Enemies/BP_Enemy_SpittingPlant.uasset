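; Spitting plant enemy Blueprint, currently with no active gameplay logic: its events are disabled stubs and the construction script only calls the parent.
; A "Position, Rotation Yaw" graph holds unconnected math for leading the player, offsetting their location along movement direction by one sixth of their distance.
; From that predicted point it derives a position 10 units from the plant toward the target and a look-at rotation.
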(fn `UserConstructionScript`
  (`parent.UserConstructionScript`))