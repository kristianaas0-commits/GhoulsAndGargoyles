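; Flying enemy character that constantly pursues the player, switching its movement component to Flying mode on BeginPlay.
; Each tick it moves horizontally toward player 0 while steering vertically toward a standard flying height.
; Within 400 units of horizontal distance it heads directly at the player in 3D instead, leaving that height.
; Movement input is scaled by MaxSpeed, and rotation snaps to face the player in yaw only.
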(event `self.ReceiveBeginPlay`
  (`parent.ReceiveBeginPlay`)
  (`CharacterMovementComponent.SetMovementMode` (`self.CharacterMovement`) "MOVE_Flying" 0))

(event `self.ReceiveTick`
  (params (DeltaSeconds :type "Float (single-precision)"))
  (bind _returnvalue (`self.K2_GetActorLocation`))
  (bind (_returnvalue_x _returnvalue_y _returnvalue_z) (`KismetMathLibrary.BreakVector` (`KismetMathLibrary.Normal` (- (`self.StandardFlyingHeight`) _returnvalue))))
  (bind _returnvalue_2 (- (`self.K2_GetActorLocation` (`GameplayStatics.GetPlayerCharacter` 0)) _returnvalue))
  (bind _returnvalue_3 (`KismetMathLibrary.Normal` _returnvalue_2))
  (bind (_returnvalue_x_2 _returnvalue_y_2) (`KismetMathLibrary.BreakVector` (`KismetMathLibrary.Normal` _returnvalue_2)))
  (bind (_returnvalue_roll _returnvalue_pitch _returnvalue_yaw) (`KismetMathLibrary.BreakRotator` (`KismetMathLibrary.Conv_VectorToRotator` _returnvalue_3)))
  ; Flying Movement and Rotation
  (if true
    (if (<= (`KismetMathLibrary.VSizeXY` _returnvalue_2) 400.0)
      (`self.AddMovementInput` _returnvalue_3 (`self.MaxSpeed`))
      (else
        (`self.AddMovementInput` (`KismetMathLibrary.MakeVector` _returnvalue_x_2 _returnvalue_y_2 _returnvalue_z) (`self.MaxSpeed`))))
    (`self.K2_SetActorRotation` (`KismetMathLibrary.MakeRotator` 0.0 0.0 _returnvalue_yaw))))

(fn `UserConstructionScript`
  (`parent.UserConstructionScript`))