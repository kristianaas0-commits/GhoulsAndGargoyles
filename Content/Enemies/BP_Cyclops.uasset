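; BP_Cyclops is a boss enemy that stays dormant until the boss wall activates.
; On BeginPlay it stops its StateTree logic, binds to the activation dispatcher of the BP_BossWall found in the level, and passes itself to its WB_CyclopsHealth widget.
; When the wall fires, it starts the StateTree, sets its Work flag and shows the health bar.
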(event `self.ReceiveBeginPlay`
  (`BrainComponent.StopLogic` (`self.StateTreeComponent`) "")
  (bind _returnvalue (`GameplayStatics.GetActorOfClass` "/Game/InteractObject/BP_BossWall.BP_BossWall_C"))
  (add `/Game/InteractObject/BP_BossWall.BossWallActivate` _returnvalue (delegate `BossWallActivate_Event`))
  (bind _aswb_cyclops_health (cast `/Game/UI/Widget/Gameplay/WB_CyclopsHealth` (`WidgetComponent.GetUserWidgetObject` (`self.Healthbar`))))
  (set `/Game/UI/Widget/Gameplay/WB_CyclopsHealth.EnemyRef` self _aswb_cyclops_health))

(event `BossWallActivate_Event`
  (`BrainComponent.StartLogic` (`self.StateTreeComponent`))
  (set `self.Work` true)
  (`SceneComponent.SetVisibility` (`self.Healthbar`) true false))

(fn `UserConstructionScript`)