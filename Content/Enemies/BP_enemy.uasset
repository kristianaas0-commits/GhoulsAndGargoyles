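; BP_enemy is an enemy actor that tracks its health and dies when damage depletes it.
; BeginPlay fills current health from MaxHealth, and AnyDamage subtracts incoming damage while health remains.
; On reaching zero, it casts player 0's character to BP_Character_FirstPerson, calls UpdateScore on it, then destroys itself.
; If that cast fails, the actor is not destroyed.
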(event `self.ReceiveBeginPlay`
  (set `self.CurrentHealth_0` (`self.MaxHealth`)))

(event `self.ReceiveAnyDamage`
  (params (Damage :type "Float (single-precision)") (DamageType :type "DamageType Object Reference") (InstigatedBy :type "Controller Object Reference") (DamageCauser :type "Actor Object Reference"))
  (bind _currenthealth_0 (`self.CurrentHealth_0`))
  ; Enemy Heath and Damage
  (if (> (`self.CurrentHealth_0`) 0.0)
    (set `self.CurrentHealth_0` (- _currenthealth_0 Damage))
    (if (<= _currenthealth_0 0.0)
      (bind _asbp_character_first_person (cast `/Game/Characters/BP_Character_FirstPerson` (`GameplayStatics.GetPlayerCharacter` 0)))
      (`/Game/Characters/BP_Character_FirstPerson.UpdateScore` _asbp_character_first_person)
      (`self.K2_DestroyActor`))))

(fn `UserConstructionScript`)