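; Enemy spawner actor that produces flying crow enemies while the player is nearby.
; Each tick it compares the 2D distance to the player character against a configurable start-spawning range.
; When in range and allowed, it spawns a crow slightly above its static mesh, then blocks further spawns behind a five-second delay cooldown.
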(event `self.ReceiveBeginPlay`)

(event `SpawnWait`
  (set `self.canSpawnEnemy` false)
  (`KismetSystemLibrary.Delay` 5.0)
  (set `self.canSpawnEnemy` true))

(event `self.ReceiveTick`
  (params (DeltaSeconds :type "Float (single-precision)"))
  (bind (_returnvalue_x _returnvalue_y) (`KismetMathLibrary.BreakVector` (`self.K2_GetActorLocation`)))
  (bind (_returnvalue_x_2 _returnvalue_y_2) (`KismetMathLibrary.BreakVector` (`self.K2_GetActorLocation` (`GameplayStatics.GetPlayerCharacter` 0))))
  (bind (_returnvalue_x_3 _returnvalue_y_3 _returnvalue_z) (`KismetMathLibrary.BreakVector` (`SceneComponent.GetSocketLocation` (`self.StaticMesh`) "None")))
  (if (<= (`KismetMathLibrary.Distance2D` (`KismetMathLibrary.MakeVector2D` _returnvalue_x_2 _returnvalue_y_2) (`KismetMathLibrary.MakeVector2D` _returnvalue_x _returnvalue_y)) (`self.DistanceBeforeStartSpawning`))
    (if (`self.canSpawnEnemy`)
      (`self.SpawnWait`)
      (`|SpawnActorFromClass` "/Game/Enemies/BP_Enemy_Flying_Crow.BP_Enemy_Flying_Crow_C" (`KismetMathLibrary.MakeTransform` (`KismetMathLibrary.MakeVector` _returnvalue_x_3 _returnvalue_y_3 (+ _returnvalue_z 50.0))) "AdjustIfPossibleButAlwaysSpawn" "MultiplyWithRoot" null null))))

(fn `UserConstructionScript`)