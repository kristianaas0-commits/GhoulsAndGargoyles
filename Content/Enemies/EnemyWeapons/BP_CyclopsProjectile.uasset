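; BP_CyclopsProjectile is an enemy weapon projectile, named for a Cyclops, that damages the player.
; BeginPlay sets the ProjectileMovement speed, turns off gravity on movement, mesh and sphere, enables mesh physics simulation, then destroys the actor after a short delay.
; When the Sphere overlaps an actor matching the player character's class, it applies fixed damage to player character 0 and destroys itself.
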(event `self.ReceiveBeginPlay`
  (bind _projectilemovement (`self.ProjectileMovement`))
  (bind _projectilemesh (`self.ProjectileMesh`))
  (set `ProjectileMovementComponent.InitialSpeed` 1500.0 _projectilemovement)
  (set `ProjectileMovementComponent.ProjectileGravityScale` 0.0 _projectilemovement)
  (`PrimitiveComponent.SetSimulatePhysics` _projectilemesh true)
  (`PrimitiveComponent.SetEnableGravity` _projectilemesh false)
  (`PrimitiveComponent.SetEnableGravity` (`self.Sphere`) false)
  (`KismetSystemLibrary.Delay` 5.0)
  (`self.K2_DestroyActor`))

(event `self.Sphere.OnComponentBeginOverlap`
  (params (OverlappedComponent :type "PrimitiveComponent Object Reference") (OtherActor :type "Actor Object Reference") (OtherComp :type "PrimitiveComponent Object Reference") (OtherBodyIndex :type Integer) (bFromSweep :type Boolean) (SweepResult :type "HitResult Structure (by ref)"))
  (bind _returnvalue (`GameplayStatics.GetPlayerCharacter` 0))
  (if (`GameplayStatics.ObjectIsA` OtherActor (`GameplayStatics.GetObjectClass` _returnvalue))
    (`GameplayStatics.ApplyDamage` _returnvalue 5.0)
    (`self.K2_DestroyActor`)))

(fn `UserConstructionScript`)