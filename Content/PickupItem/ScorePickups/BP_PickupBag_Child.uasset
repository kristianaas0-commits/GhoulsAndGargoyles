(event `self.ReceiveBeginPlay`
  (`parent.ReceiveBeginPlay`))

(fn `Do your thing`
  (bind (_s_pickup_coin_isgolem _s_pickup_coin_score) (break `/Game/PickupItem/ScorePickups/S_PickupScoreItems` (`self.S Pickup Coin`)))
  (bind _asjarl_third_person_character_cpp (cast `Jarl_ThirdPersonCharacter_CPP` (`GameplayStatics.GetPlayerCharacter` 0)))
  (`Jarl_ThirdPersonCharacter_CPP.UpdateScore` _asjarl_third_person_character_cpp _s_pickup_coin_score _s_pickup_coin_isgolem)
  (`GameplayStatics.PlaySoundAtLocation` "/Engine/EngineSounds/1kSineTonePing.1kSineTonePing" (`self.K2_GetActorLocation`) (struct) 1.0 1.0 0.0 null null null null))

(fn `UserConstructionScript`
  (`parent.UserConstructionScript`))