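; BP_BossWall is a barrier that seals behind the player and clears other enemies for what appears to be the Cyclops boss fight.
; Its Cube starts with collision disabled on BeginPlay.
; When an actor of the player character's class overlaps the Box, it destroys every EnemyParent actor in the level except BP_Cyclops.
; After a short delay, the Cube enables query and physics collision.
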(event `self.ReceiveBeginPlay`
  (`PrimitiveComponent.SetCollisionEnabled` (`self.Cube`) "NoCollision"))

(event `self.Box.OnComponentBeginOverlap`
  (params (OverlappedComponent :type "PrimitiveComponent Object Reference") (OtherActor :type "Actor Object Reference") (OtherComp :type "PrimitiveComponent Object Reference") (OtherBodyIndex :type Integer) (bFromSweep :type Boolean) (SweepResult :type "HitResult Structure (by ref)"))
  (if (`GameplayStatics.ObjectIsA` OtherActor (`GameplayStatics.GetObjectClass` (`GameplayStatics.GetPlayerCharacter` 0)))
    (bind _outactors (`GameplayStatics.GetAllActorsOfClass` "/Script/GnG.EnemyParent"))
    (for _array_element _outactors
      (if (not (`GameplayStatics.ObjectIsA` _array_element "/Game/Enemies/BP_Cyclops.BP_Cyclops_C"))
        (`self.K2_DestroyActor` _array_element)))
    (`KismetSystemLibrary.Delay` 0.2)
    (`PrimitiveComponent.SetCollisionEnabled` (`self.Cube`) "QueryAndPhysics")))

(fn `UserConstructionScript`)